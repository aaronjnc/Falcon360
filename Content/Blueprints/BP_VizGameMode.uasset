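; Game mode that builds a split-screen ring of local-player cameras around one parent pawn, with Panini projection set by console commands in construction.
; BeginPlay spawns a split-screen manager and requests indexed local players through VizStudioGameInstance.
; It swaps the first player's receiver pawn for a BP_VizParentPawn at PlayerStart.
; The remaining receivers are yawed at 45-degree steps, attached to that parent, and their audio listeners overridden to its root.
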(event `self.ReceiveBeginPlay`
  (bind _returnvalue (`GameplayStatics.GetPlayerController` 0))
  (`|SpawnActorFromClass` "/Script/Falcon360.ASplitScreenManager" (`KismetMathLibrary.MakeTransform` (0.0 0.0 0.0)) "Undefined" "OverrideRootScale" null null)
  (for _index (range 9)
    (bind _asviz_studio_game_instance (cast `VizStudioGameInstance` (`GameplayStatics.GetGameInstance`)))
    (`VizStudioGameInstance.RequestLocalPlayer` _asviz_studio_game_instance _index true))
  (`Controller.UnPossess` _returnvalue)
  (bind _outactors (`GameplayStatics.GetAllActorsOfClass` "/Game/Blueprints/BP_VizCameraReceiverPawn.BP_VizCameraReceiverPawn_C"))
  (`self.K2_DestroyActor` (`|GetArrayItem` _outactors))
  (bind _returnvalue_2 (`GameplayStatics.GetActorOfClass` "/Script/Engine.PlayerStart"))
  (bind _returnvalue_3 (`|SpawnActorFromClass` "/Game/Blueprints/BP_VizParentPawn.BP_VizParentPawn_C" (`self.GetTransform` _returnvalue_2) "Undefined" "OverrideRootScale" null null))
  (`Controller.Possess` _returnvalue _returnvalue_3)
  (bind _outactors_2 (`GameplayStatics.GetAllActorsOfClass` "/Game/Blueprints/BP_VizCameraReceiverPawn.BP_VizCameraReceiverPawn_C"))
  (for (_array_element _array_index) _outactors_2
    (`self.K2_SetActorRotation` _array_element (`KismetMathLibrary.MakeRotator` 0.0 0.0 (+ (* _array_index 45.0) 202.5)) false)
    (bind _returnvalue_4 (`GameplayStatics.GetActorOfClass` "/Game/Blueprints/BP_VizParentPawn.BP_VizParentPawn_C"))
    (`self.K2_AttachToActor` _array_element _returnvalue_4 "None" "KeepRelative" "KeepRelative" "KeepRelative" true)
    (`PlayerController.SetAudioListenerOverride` :`self` (cast `PlayerController` (`Pawn.GetController` _array_element) :!pure true) :`AttachToComponent` (`Actor.RootComponent` _returnvalue_4))))

(fn `UserConstructionScript`
  (`KismetSystemLibrary.ExecuteConsoleCommand` "r.Upscale.Panini.D 1" null)
  (`KismetSystemLibrary.ExecuteConsoleCommand` "r.Upscale.Panini.S -0.5" null)
  (`KismetSystemLibrary.ExecuteConsoleCommand` "r.Upscale.Panini.ScreenFit 1.95" null))