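; Parent pawn for a multi-camera viz rig that spawns its own BP_VizPlayerController on BeginPlay and gathers all BP_VizCameraReceiverPawn cameras when possessed.
; MovementCameraDarkening rounds movement axes into eight directions, keeping a camera pair at normal exposure and darkening the rest through post-process settings.
; Idle restores exposure, and the blur material's weight is always zero.
; The movement input and darkening calls are disconnected in the event graph.
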(event `self.ReceiveBeginPlay`
  (bind _returnvalue (`|SpawnActorFromClass` "/Game/Blueprints/BP_VizPlayerController.BP_VizPlayerController_C" (`self.GetTransform`) "Undefined" "OverrideRootScale" null null))
  (`Controller.Possess` _returnvalue self))

(event `self.ReceivePossessed`
  (params (NewController :type "Controller Object Reference"))
  (bind _outactors (`GameplayStatics.GetAllActorsOfClass` "/Game/Blueprints/BP_VizCameraReceiverPawn.BP_VizCameraReceiverPawn_C"))
  (bind _output_get (set `self.VizCameraPawns` _outactors))
  (for _array_element _output_get
    (`KismetArrayLibrary.Array_AddUnique` (`self.CameraRefs`) (`/Game/Blueprints/BP_VizCameraReceiverPawn.Camera` _array_element)))
  (`KismetSystemLibrary.PrintString` "Possessed"))

(fn `DirectionalCamDarken`
  (params (Cam1 :type Integer) (Cam2 :type Integer))
  (locals (DarkenedCameras :type "Array of CameraComponent Object Reference"))
  (bind _camerarefs (`self.CameraRefs`))
  (bind _darkenedcameras (`local.DarkenedCameras`))
  (bind _output (`|GetArrayItem` _camerarefs Cam1))
  (bind _output_2 (`|GetArrayItem` _camerarefs Cam2))
  (set `local.DarkenedCameras` _camerarefs)
  (setmembers `PostProcessSettings` :`StructRef` (`CameraComponent.PostProcessSettings` _output) :`AutoExposureBias` 0.0)
  (setmembers `PostProcessSettings` :`StructRef` (`CameraComponent.PostProcessSettings` _output_2) :`AutoExposureBias` 0.0 :`WeightedBlendables` (make `WeightedBlendables` (`|MakeArray` (make `WeightedBlendable` 0.0 "/Game/Assets/Materials/M_Blur_PP.M_Blur_PP"))))
  (`KismetArrayLibrary.Array_RemoveItem` _darkenedcameras _output)
  (`KismetArrayLibrary.Array_RemoveItem` _darkenedcameras _output_2)
  (for _array_element (`local.DarkenedCameras`)
    (setmembers `PostProcessSettings` :`StructRef` (`CameraComponent.PostProcessSettings` _array_element) :`AutoExposureBias` -3.0 :`WeightedBlendables` (make `WeightedBlendables` (`|MakeArray` (make `WeightedBlendable` 0.0 "/Game/Assets/Materials/M_Blur_PP.M_Blur_PP"))))))

(fn `MovementCameraDarkening`
  (params (`Right/Left` :type "Float (double-precision)") (`Forward/Back` :type "Float (double-precision)"))
  (bind _returnvalue (`KismetStringLibrary.Concat_StrStr` (`KismetStringLibrary.Conv_IntToString` (`KismetMathLibrary.Round` (`KismetMathLibrary.Dot_VectorVector` (`KismetMathLibrary.MakeVector` 0.0 `Right/Left`) (0.0 1.0 0.0)))) "" (`KismetStringLibrary.Conv_IntToString` (`KismetMathLibrary.Round` (`KismetMathLibrary.Dot_VectorVector` (`KismetMathLibrary.MakeVector` `Forward/Back`) (1.0 0.0 0.0))))))
  (if (not (`KismetStringLibrary.EqualEqual_StrStr` _returnvalue (`self.CurrentDirection`)))
    (bind _output_get (set `self.CurrentDirection` _returnvalue))
    (set `self.FadeComplete` false)
    (switch `string` _output_get
      (:`0,0`
        (for _array_element (`self.CameraRefs`)
          (setmembers `PostProcessSettings` :`StructRef` (`CameraComponent.PostProcessSettings` _array_element) :`AutoExposureBias` 0.0 :`WeightedBlendables` (make `WeightedBlendables` (`|MakeArray` (make `WeightedBlendable` 0.0 "/Game/Assets/Materials/M_Blur_PP.M_Blur_PP"))))))
      (:`0,-1`
        (`self.DirectionalCamDarken` 7))
      (:`-1,-1`
        (`self.DirectionalCamDarken` 0 1))
      (:`-1,0`
        (`self.DirectionalCamDarken` 1 2))
      (:`-1,1`
        (`self.DirectionalCamDarken` 2 3))
      (:`0,1`
        (`self.DirectionalCamDarken` 3 4))
      (:`1,1`
        (`self.DirectionalCamDarken` 4 5))
      (:`1,0`
        (`self.DirectionalCamDarken` 5 6))
      (:`1,-1`
        (`self.DirectionalCamDarken` 6 7)))))

(fn `UserConstructionScript`)