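; BP_VizParentPawn is a pawn that sets up its own player controller and gathers references to the VisStudio camera pawns.
; On BeginPlay it spawns a BP_VizPlayerController to possess itself, then adds IMC_Default to player controller 0's Enhanced Input subsystem.
; On possession it collects all BP_VizCameraReceiverPawn actors and their cameras.
; IA_Rotate drives controller yaw, and unpossession only prints a debug message.
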(event `self.ReceiveBeginPlay`
  (bind _returnvalue (pcsubsystem `EnhancedInputLocalPlayerSubsystem` (`GameplayStatics.GetPlayerController` 0)))
  (bind _returnvalue_2 (`|SpawnActorFromClass` "/Game/Blueprints/VisStudio/BP_VizPlayerController.BP_VizPlayerController_C" (`self.GetTransform`) "Undefined" "OverrideRootScale" null null))
  (`Controller.Possess` _returnvalue_2 self)
  (`/Engine/EditorBlueprintResources/StandardMacros.IsValid` _returnvalue
    (:`Is Valid`
      (`EnhancedInputSubsystemInterface.AddMappingContext` _returnvalue "/Game/Input/IMC_Default.IMC_Default" 0 (struct)))))

(event `EnhancedInput|/Game/Input/Actions/IA_Rotate`
  (params (ActionValue :type "Float (double-precision)") (ElapsedSeconds :type "Float (double-precision)") (TriggeredSeconds :type "Float (double-precision)") (InputAction :type "InputAction Object Reference" :default "/Game/Input/Actions/IA_Rotate.IA_Rotate"))
  (:`Triggered`
    (`self.AddControllerYawInput` ActionValue)))

(event `self.ReceivePossessed`
  (params (NewController :type "Controller Object Reference"))
  (bind _outactors (`GameplayStatics.GetAllActorsOfClass` "/Game/Blueprints/VisStudio/BP_VizCameraReceiverPawn.BP_VizCameraReceiverPawn_C"))
  (bind _output_get (set `self.VizCameraPawns` _outactors))
  (for _array_element _output_get
    (`KismetArrayLibrary.Array_AddUnique` (`self.CameraRefs`) (`/Game/Blueprints/VisStudio/BP_VizCameraReceiverPawn.Camera` _array_element))))

(event `self.ReceiveUnpossessed`
  (params (OldController :type "Controller Object Reference"))
  (`KismetSystemLibrary.PrintString` "Unpossess"))

(fn `UserConstructionScript`)